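; Scarry is a monster character that reacts to spotting the player with threaten, roar and fighting montages.
; PawnSensing flags the player as close, and Tick then starts the guarded montage sequence, chained with delays equal to each montage's length.
; The fighting montage loops while the player stays within range, then both flags reset.
; Mesh collision follows CollisionEnable at BeginPlay, which the construction script sets to off.
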(event `self.ReceiveBeginPlay`
  (`PrimitiveComponent.SetCollisionEnabled` (`self.Mesh`) (select `bool` (`self.Collision Enable`) :`false` "NoCollision" :`true` "QueryAndPhysics" :!type "ECollisionEnabled Enum")))

(event `self.ReceiveTick`
  (params (DeltaSeconds :type "Float (single-precision)"))
  (if (`self.IsPlayerClose`)
    (if (not (`self.IsAttacking`))
      (set `self.IsAttacking` true)
      (`KismetSystemLibrary.PrintString` "Roar")
      (bind _returnvalue (`self.PlayAnimMontage` "/Game/Character/monster/Scarry/Scarry_Theaten_Montage.Scarry_Theaten_Montage"))
      (`KismetSystemLibrary.Delay` _returnvalue)
      (bind _returnvalue_2 (`self.PlayAnimMontage` "/Game/Character/monster/Scarry/Scarry_Roaring_Montage.Scarry_Roaring_Montage"))
      (`KismetSystemLibrary.Delay` _returnvalue_2)
      (if (<= (`self.GetDistanceTo` (cast `/Game/Character/Mesh/CharacterTP_BP` (`GameplayStatics.GetPlayerCharacter` 0) :!pure true)) 900.0) :!label _label
        (bind _returnvalue_3 (`self.PlayAnimMontage` "/Game/Character/monster/Scarry/Scarry_Fighting_Montage.Scarry_Fighting_Montage"))
        (`KismetSystemLibrary.Delay` _returnvalue_3)
        (goto _label)
        (else
          (set `self.IsAttacking` false)
          (set `self.IsPlayerClose` false)
          (`KismetSystemLibrary.PrintString` "Stop Roar"))))))

(event `self.PawnSensing.OnSeePawn`
  (params (Pawn :type "Pawn Object Reference"))
  (bind _ascharacter_tp_bp (cast `/Game/Character/Mesh/CharacterTP_BP` Pawn))
  (`/Engine/EditorBlueprintResources/StandardMacros.IsValid` _ascharacter_tp_bp
    (:`Is Valid`
      (set `self.IsPlayerClose` true)
      (`KismetSystemLibrary.PrintString` "Say Hello to Lucas"))))

(fn `UserConstructionScript`
  (set `self.Collision Enable` false))