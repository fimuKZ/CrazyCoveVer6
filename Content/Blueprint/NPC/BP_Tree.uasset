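; BP_Tree is an interactable NPC pawn that starts a dialogue with the player.
; On BeginPlay it hands its DialougeTree to its AI_NPC controller, which runs the conversation.
; Interact calls StartDialogue on that controller, then hides the first top-level WB_CharacterHUD widget; this Blueprint never shows it again.
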(event `self.ReceiveBeginPlay`
  (bind _dialougetree (`self.DialougeTree`))
  (set `/Game/Blueprint/NPC/AI_NPC.DialougeTree` _dialougetree (cast `/Game/Blueprint/NPC/AI_NPC` (`AIBlueprintHelperLibrary.GetAIController` self) :!pure true))
  (set `self.DialougeTree` _dialougetree))

(event `Event Interact`
  (`/Game/Blueprint/NPC/AI_NPC.Start Dialogue` (cast `/Game/Blueprint/NPC/AI_NPC` (`AIBlueprintHelperLibrary.GetAIController` self) :!pure true))
  (bind _foundwidgets (`WidgetBlueprintLibrary.GetAllWidgetsOfClass` "/Game/UI/Blueprint/WB_CharacterHUD.WB_CharacterHUD_C"))
  (`Widget.SetVisibility` (`|GetArrayItem` _foundwidgets) "Hidden"))

(fn `UserConstructionScript`)