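; AI controller Blueprint for NPCs that drives dialogue through a behavior tree.
; StartDialogue runs the dialogue tree, and EndDialogue stops the brain logic and makes the character HUD widget visible again.
; When the IsFastTravel flag is set, ending dialogue also toggles the HUD's map.
; A UI-only input and mouse cursor block is left unconnected.
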(event `Start Dialogue`
  (`self.RunBehaviorTree` (`self.DialougeTree`)))

(event `End Dialogue`
  (`BrainComponent.StopLogic` (`self.BrainComponent`) "")
  (bind _foundwidgets (`WidgetBlueprintLibrary.GetAllWidgetsOfClass` "/Game/UI/Blueprint/WB_CharacterHUD.WB_CharacterHUD_C"))
  (`Widget.SetVisibility` (`|GetArrayItem` _foundwidgets) "Visible")
  (if (`self.isFastTravel`)
    (bind _foundwidgets_2 (`WidgetBlueprintLibrary.GetAllWidgetsOfClass` "/Game/UI/Blueprint/WB_CharacterHUD.WB_CharacterHUD_C"))
    (`/Game/UI/Blueprint/WB_CharacterHUD.ToggleMap` (`|GetArrayItem` _foundwidgets_2))))

(fn `UserConstructionScript`)