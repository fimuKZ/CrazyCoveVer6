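; Behavior Tree task that opens the dialogue box when a conversation with an NPC starts.
; It casts the controlled pawn to BP_NPC and fills the game mode's InteractUI dialogue widget with that NPC's name and portrait, then shows it.
; It stores the widget in the Blackboard, disables player input, shows the mouse cursor and finishes successfully.
; A failed cast stops execution without calling FinishExecute.
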(event `self.ReceiveExecuteAI`
  (params (OwnerController :type "AIController Object Reference") (ControlledPawn :type "Pawn Object Reference"))
  (bind _returnvalue (`GameplayStatics.GetPlayerController` 0))
  (bind _npcpawn (`self.NPCpawn`))
  (bind _asbp_npc (cast `/Game/Blueprint/NPC/BP_NPC` ControlledPawn))
  (set `self.NPCpawn` _asbp_npc)
  (bind _asthird_person_game_mode (cast `/Game/ThirdPersonBP/Blueprints/ThirdPersonGameMode` (`GameplayStatics.GetGameMode`)))
  (bind _wb_dialougebox (`/Game/Blueprint/Interaction_Interfaces/WB_InteractUI.WB_DialougeBox` (`/Game/ThirdPersonBP/Blueprints/ThirdPersonGameMode.InteractUI` _asthird_person_game_mode)))
  (set `/Game/Blueprint/Interaction_Interfaces/WB_DialougeBox.SpeakerName` (`/Game/Blueprint/NPC/BP_NPC.Name` _npcpawn) _wb_dialougebox)
  (`Image.SetBrushFromTexture` (`/Game/Blueprint/Interaction_Interfaces/WB_DialougeBox.ProfilePicture` _wb_dialougebox) (`/Game/Blueprint/NPC/BP_NPC.ProfilePicture` _npcpawn) true)
  (`Widget.SetVisibility` _wb_dialougebox "Visible")
  (`BTFunctionLibrary.SetBlackboardValueAsObject` (`self.BB_DialogueUI`) _wb_dialougebox)
  (`Actor.DisableInput` (`GameplayStatics.GetPlayerCharacter` 0) _returnvalue)
  (set `PlayerController.bShowMouseCursor` true _returnvalue)
  (`self.FinishExecute` true))