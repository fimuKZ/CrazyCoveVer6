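; Behavior tree task that closes an NPC dialogue and returns control to the player.
; It reads the dialogue widget from the blackboard, hides it, then calls EndDialogue on the owning AI_NPC controller.
; It then shows the mouse cursor, re-enables player character input and finishes successfully.
; If either cast fails, execution stops without calling FinishExecute.
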(event `self.ReceiveExecuteAI`
  (params (OwnerController :type "AIController Object Reference") (ControlledPawn :type "Pawn Object Reference"))
  (bind _returnvalue (`GameplayStatics.GetPlayerController` 0))
  (bind _aswidget (cast `Widget` (`BTFunctionLibrary.GetBlackboardValueAsObject` (`self.BB_dialogueUI`))))
  (`Widget.SetVisibility` _aswidget "Hidden")
  (bind _asai_npc (cast `/Game/Blueprint/NPC/AI_NPC` OwnerController))
  (`/Game/Blueprint/NPC/AI_NPC.End Dialogue` _asai_npc)
  (set `PlayerController.bShowMouseCursor` true _returnvalue)
  (`Actor.EnableInput` (`GameplayStatics.GetPlayerCharacter` 0) _returnvalue)
  (`self.FinishExecute` true))